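; BP_RoofTiles is a kit-bash environment actor that procedurally builds a two-sided tiled roof from width and length parameters.
; The construction script derives row count from RoofWidth and adds mirrored tile instances stepping down each slope, with slight random jitter.
; It then scales a background plane for each side, mirroring the left via negative X, and spaces top beam instances along the ridge.
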(fn `GetBeamTransform`
  (params (Index :type Integer))
  (returns (Transform :type "Transform Structure"))
  (return (`KismetMathLibrary.MakeTransform` (`KismetMathLibrary.MakeVector` 0.0 (`KismetMathLibrary.Conv_IntToDouble` (* Index 150))) (struct :`Yaw` 180.0))))

(fn `GetLeftTransform`
  (params (Index :type Integer))
  (returns (Transform :type "Transform Structure"))
  (locals (MultiplyFactor :type Integer :default 50) (XZOffset :type "Float (double-precision)"))
  (set `local.XZOffset` (`KismetMathLibrary.RandomFloatInRange` -2.0 2.0))
  (return (`KismetMathLibrary.MakeTransform` (`KismetMathLibrary.MakeVector` (+ (`local.XZOffset`) (* (`KismetMathLibrary.Conv_IntToDouble` (`self.CurrentLevel`)) (`local.MultiplyFactor`))) (* (`self.LengthOfTile`) Index 100.0) (+ (`local.XZOffset`) (* (`KismetMathLibrary.Conv_IntToDouble` (`self.CurrentLevel`)) -0.652 (`local.MultiplyFactor`)))) (struct))))

(fn `GetRightTransform`
  (params (Index :type Integer))
  (returns (Transform :type "Transform Structure"))
  (locals (MultiplyFactor :type Integer :default 50) (XZOffset :type "Float (double-precision)"))
  (set `local.XZOffset` (`KismetMathLibrary.RandomFloatInRange` -2.0 2.0))
  (return (`KismetMathLibrary.MakeTransform` (`KismetMathLibrary.MakeVector` (+ (`local.XZOffset`) (* (`KismetMathLibrary.Conv_IntToDouble` (`self.CurrentLevel`)) (`local.MultiplyFactor`) -1.0)) (* (`self.LengthOfTile`) Index 100.0) (+ (`local.XZOffset`) (* (`KismetMathLibrary.Conv_IntToDouble` (`self.CurrentLevel`)) -0.652 (`local.MultiplyFactor`)))) (struct :`Yaw` 180.0))))

(fn `PopulateBeams`
  (for _index (range (+ (/ (`self.RoofLength`) 3) 1))
    (`InstancedStaticMeshComponent.AddInstance` (`self.TopBeam`) (`self.GetBeamTransform` _index) false)))

(fn `PopulateRow`
  (for _index (range (`self.RoofLength`))
    (`InstancedStaticMeshComponent.AddInstance` (`self.RoofTile`) (`self.GetRightTransform` _index) false)
    (`InstancedStaticMeshComponent.AddInstance` (`self.RoofTile`) (`self.GetLeftTransform` _index) false)))

(fn `ResizeBackgroundLeft`
  (bind _returnvalue (`KismetMathLibrary.Conv_IntToDouble` (`self.RoofLevels`)))
  (`SceneComponent.SetWorldScale3D` (`self.BackgroundPlaneLeft`) (`KismetMathLibrary.MakeVector` (* _returnvalue -1.0) (`KismetMathLibrary.Conv_IntToDouble` (`self.RoofLength`)) _returnvalue)))

(fn `ResizeBackgroundRight`
  (bind _returnvalue (`KismetMathLibrary.Conv_IntToDouble` (`self.RoofLevels`)))
  (`SceneComponent.SetWorldScale3D` (`self.BackgroundPlaneRight`) (`KismetMathLibrary.MakeVector` _returnvalue (`KismetMathLibrary.Conv_IntToDouble` (`self.RoofLength`)) _returnvalue)))

(fn `UserConstructionScript`
  (set `self.RoofLevels` (* (`self.RoofWidth`) 3))
  (for _ (range (`self.RoofLevels`))
    (`self.PopulateRow`)
    (`/Engine/EditorBlueprintResources/StandardMacros.IncrementInt` (`self.CurrentLevel`)))
  (`self.ResizeBackgroundRight`)
  (`self.ResizeBackgroundLeft`)
  (`self.PopulateBeams`))