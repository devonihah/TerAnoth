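; Procedural kit-bash house actor that assembles modular static-mesh walls in its Construction Script, sized from mesh bounds and tile counts.
; Each bottom-floor side gets randomized wall style, door, optional door cover, corner post and optional bump-out with offset end meshes.
; StopLogic freezes randomization by rebuilding from stored per-side mesh and transform data.
; Upper floors are unfinished: the height loop is empty and CreateUpperLevels is never called.
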(fn `AddCornerPost`
  (params (HouseSides :type "/Game/Environment/KitBash/Blueprints/ENUM_HouseSides Enum" :default "NewEnumerator0"))
  (locals (RelativeTransform :type "Transform Structure"))
  (switch `/Game/Environment/KitBash/Blueprints/ENUM_HouseSides` HouseSides
    (:`NewEnumerator0`
      (set `local.RelativeTransform` (`KismetMathLibrary.MakeTransform` (`KismetMathLibrary.MakeVector` (`KismetMathLibrary.Conv_IntToDouble` (* (`self.LengthOfHouse`) (`self.LengthOfOneTile`))) (`KismetMathLibrary.Conv_IntToDouble` (* (`self.WidthOfHouse`) (`self.LengthOfOneTile`)))))))
    (:`NewEnumerator1`
      (set `local.RelativeTransform` (`KismetMathLibrary.MakeTransform` (0.0 0.0 0.0))))
    (:`NewEnumerator2`
      (set `local.RelativeTransform` (`KismetMathLibrary.MakeTransform` (`KismetMathLibrary.MakeVector` 0.0 (`KismetMathLibrary.Conv_IntToDouble` (* (`self.WidthOfHouse`) (`self.LengthOfOneTile`)))))))
    (:`NewEnumerator3`
      (set `local.RelativeTransform` (`KismetMathLibrary.MakeTransform` (`KismetMathLibrary.MakeVector` (`KismetMathLibrary.Conv_IntToDouble` (* (`self.LengthOfHouse`) (`self.LengthOfOneTile`))))))))
  (`AddComponent|NODE_AddStaticMeshComponent-13` :`RelativeTransform` (`local.RelativeTransform`)))

(fn `AddOffsetMeshes`
  (params (HouseSide :type "/Game/Environment/KitBash/Blueprints/ENUM_HouseSides Enum" :default "NewEnumerator0"))
  (locals (FirstTransform :type "Transform Structure") (SecondTransform :type "Transform Structure") (OffsetStaticMesh :type "StaticMesh Object Reference"))
  (bind _bottomflooroffsetoptions (`self.BottomFloorOffsetOptions`))
  (if (`|GetArrayItem` (`self.BottomFloorSideIsOffset`) (select `/Game/Environment/KitBash/Blueprints/ENUM_HouseSides` HouseSide :`NewEnumerator1` 1 :`NewEnumerator2` 2 :`NewEnumerator3` 3))
    (`|ExecutionSequence`
      (:`then_0`
        (switch `/Game/Environment/KitBash/Blueprints/ENUM_HouseSides` (`local.HouseSide`)
          (:`NewEnumerator0`
            (set `local.FirstTransform` (`KismetMathLibrary.MakeTransform` (`KismetMathLibrary.MakeVector` (`KismetMathLibrary.Conv_IntToDouble` (`self.LengthOfOneTile`)) (`KismetMathLibrary.Conv_IntToDouble` (* (`self.WidthOfHouse`) (`self.LengthOfOneTile`)))) (struct :`Yaw` 90.0)))
            (set `local.SecondTransform` (`KismetMathLibrary.MakeTransform` (`KismetMathLibrary.MakeVector` (`KismetMathLibrary.Conv_IntToDouble` (* (`self.LengthOfOneTile`) (- (`self.LengthOfHouse`) 1))) (`KismetMathLibrary.Conv_IntToDouble` (* (`self.WidthOfHouse`) (`self.LengthOfOneTile`)))) (struct :`Yaw` 90.0))))
          (:`NewEnumerator1`
            (set `local.FirstTransform` (`KismetMathLibrary.MakeTransform` (`KismetMathLibrary.MakeVector` (`KismetMathLibrary.Conv_IntToDouble` (`self.LengthOfOneTile`))) (struct :`Yaw` -90.0)))
            (set `local.SecondTransform` (`KismetMathLibrary.MakeTransform` (`KismetMathLibrary.MakeVector` (`KismetMathLibrary.Conv_IntToDouble` (* (`self.LengthOfOneTile`) (- (`self.LengthOfHouse`) 1)))) (struct :`Yaw` -90.0))))
          (:`NewEnumerator2`
            (set `local.FirstTransform` (`KismetMathLibrary.MakeTransform` (`KismetMathLibrary.MakeVector` (`KismetMathLibrary.Conv_IntToDouble` (* (`self.LengthOfHouse`) (`self.LengthOfOneTile`))) (`KismetMathLibrary.Conv_IntToDouble` (`self.LengthOfOneTile`)))))
            (set `local.SecondTransform` (`KismetMathLibrary.MakeTransform` (`KismetMathLibrary.MakeVector` (`KismetMathLibrary.Conv_IntToDouble` (* (`self.LengthOfHouse`) (`self.LengthOfOneTile`))) (`KismetMathLibrary.Conv_IntToDouble` (* (- (`self.WidthOfHouse`) 1) (`self.LengthOfOneTile`)))))))
          (:`NewEnumerator3`
            (set `local.FirstTransform` (`KismetMathLibrary.MakeTransform` (`KismetMathLibrary.MakeVector` 0.0 (`KismetMathLibrary.Conv_IntToDouble` (`self.LengthOfOneTile`))) (struct :`Yaw` -180.0)))
            (set `local.SecondTransform` (`KismetMathLibrary.MakeTransform` (`KismetMathLibrary.MakeVector` 0.0 (`KismetMathLibrary.Conv_IntToDouble` (* (- (`self.WidthOfHouse`) 1) (`self.LengthOfOneTile`)))) (struct :`Yaw` -180.0))))))
      (:`then_1`
        (`|ExecutionSequence`
          (:`then_0`
            (bind _returnvalue (`AddComponent|NODE_AddStaticMeshComponent-18` :`RelativeTransform` (`local.FirstTransform`)))
            (bind _output_get (set `local.OffsetStaticMesh` (`|GetArrayItem` _bottomflooroffsetoptions (`KismetMathLibrary.RandomIntegerInRange` 0 (- (`KismetArrayLibrary.Array_Length` _bottomflooroffsetoptions) 1)))))
            (`StaticMeshComponent.SetStaticMesh` _returnvalue _output_get))
          (:`then_1`
            (bind _returnvalue_2 (`AddComponent|NODE_AddStaticMeshComponent-20` :`RelativeTransform` (`local.SecondTransform`)))
            (`StaticMeshComponent.SetStaticMesh` _returnvalue_2 (`local.OffsetStaticMesh`))))))))

(fn `CreateBottomFloorSide`
  (params (HouseSide :type "/Game/Environment/KitBash/Blueprints/ENUM_HouseSides Enum" :default "NewEnumerator0"))
  (locals (RelativeTransform :type "Transform Structure") (NumTilesToMake :type Integer) (Index :type Integer) (LastDoorIndex :type Integer :default 3) (RandomDoorSpot :type Integer :default 0) (RandomDoorStyle :type Integer :default 0) (bDoorHasBeenCreated :type Boolean) (bDontUseBraces :type Boolean) (bUseOffset :type Boolean) (bUseDoorCover :type Boolean) (DoorStaticMesh :type "StaticMesh Object Reference"))
  (bind _numtilestomake (`local.NumTilesToMake`))
  (bind (_bottomfloorsides_northwall _bottomfloorsides_southwall _bottomfloorsides_eastwall _bottomfloorsides_westwall) (break `/Game/Environment/KitBash/Blueprints/STR_SideArrays` (`self.BottomFloorSides`)))
  (bind (_bottomfloorsides_northwall_2 _bottomfloorsides_southwall_2 _bottomfloorsides_eastwall_2 _bottomfloorsides_westwall_2) (break `/Game/Environment/KitBash/Blueprints/STR_SideArrays` (`self.BottomFloorSides`)))
  (bind (_bottomfloorsides_northwall_3 _bottomfloorsides_southwall_3 _bottomfloorsides_eastwall_3 _bottomfloorsides_westwall_3) (break `/Game/Environment/KitBash/Blueprints/STR_SideArrays` (`self.BottomFloorSides`)))
  (bind (_bottomfloordoorcovers_northwall _bottomfloordoorcovers_southwall _bottomfloordoorcovers_eastwall _bottomfloordoorcovers_westwall) (break `/Game/Environment/KitBash/Blueprints/STR_SideTile` (`self.BottomFloorDoorCovers`)))
  (bind (_bottomfloordoorcovers_northwall_2 _bottomfloordoorcovers_southwall_2 _bottomfloordoorcovers_eastwall_2 _bottomfloordoorcovers_westwall_2) (break `/Game/Environment/KitBash/Blueprints/STR_SideTile` (`self.BottomFloorDoorCovers`)))
  (bind _houseside (`local.HouseSide`))
  (bind _returnvalue (- (`self.LengthOfHouse`) 1))
  (bind _returnvalue_2 (- (`self.WidthOfHouse`) 1))
  (bind _output_mesh (break `/Game/Environment/KitBash/Blueprints/STR_MeshWithTransform` (`|GetArrayItem` (select `/Game/Environment/KitBash/Blueprints/ENUM_HouseSides` (`local.HouseSide`) :`NewEnumerator0` _bottomfloorsides_northwall_2 :`NewEnumerator1` _bottomfloorsides_southwall_2 :`NewEnumerator2` _bottomfloorsides_eastwall_2 :`NewEnumerator3` _bottomfloorsides_westwall_2) (`local.Index`))))
  ;[0 1 0] Set all of the random variables for side variations
  (set `local.bUseDoorCover` (`KismetMathLibrary.RandomBoolWithWeight` 0.66))
  (set `local.bDontUseBraces` (`KismetMathLibrary.RandomBool`))
  (bind _output_get (set `local.bUseOffset` (`KismetMathLibrary.RandomBoolWithWeight` 0.333)))
  (`self.AddCornerPost` (`local.HouseSide`))
  (`KismetArrayLibrary.Array_Set` (`self.BottomFloorSideIsOffset`) (select `/Game/Environment/KitBash/Blueprints/ENUM_HouseSides` (`local.HouseSide`) :`NewEnumerator1` 1 :`NewEnumerator2` 2 :`NewEnumerator3` 3) _output_get)
  ;[0 1 0] Set the number of tiles to make based on the cardinal direction and the corresponding length or width
  (switch `/Game/Environment/KitBash/Blueprints/ENUM_HouseSides` (`local.HouseSide`)
    (:`NewEnumerator0`
      (set `local.NumTilesToMake` _returnvalue))
    (:`NewEnumerator1`
      (set `local.NumTilesToMake` _returnvalue))
    (:`NewEnumerator2`
      (set `local.NumTilesToMake` _returnvalue_2))
    (:`NewEnumerator3`
      (set `local.NumTilesToMake` _returnvalue_2)))
  (for _index (range (+ _numtilestomake 1))
    (set `local.Index` _index)
    (bind _transform (`self.SetTransformFromHouseSide` (`local.HouseSide`) (`local.Index`) (`local.bUseOffset`) _numtilestomake))
    (bind _output_get_2 (set `local.RelativeTransform` _transform))
    (bind _returnvalue_3 (`AddComponent|NODE_AddStaticMeshComponent-8` :`RelativeTransform` _output_get_2))
    (`|ExecutionSequence`
      (:`then_0`
        ;[0 1 0] Add the random tile to the correct BottomFloorSides array
        (`KismetArrayLibrary.Array_Add` (select `/Game/Environment/KitBash/Blueprints/ENUM_HouseSides` (`local.HouseSide`) :`NewEnumerator0` _bottomfloorsides_northwall :`NewEnumerator1` _bottomfloorsides_southwall :`NewEnumerator2` _bottomfloorsides_eastwall :`NewEnumerator3` _bottomfloorsides_westwall) (make `/Game/Environment/KitBash/Blueprints/STR_MeshWithTransform` (`|GetArrayItem` (`self.BottomFloorOptions`) (`KismetMathLibrary.SelectInt` 4 5 (`local.bDontUseBraces`))) (`local.RelativeTransform`))))
      (:`then_1`
        ;[0 1 0] Set the static mesh just added to the StaticMeshComponent array to the one added to the BottomFloorSides array
        (`StaticMeshComponent.SetStaticMesh` _returnvalue_3 _output_mesh))))
  (set `local.RandomDoorStyle` (`KismetMathLibrary.SelectInt` (`KismetMathLibrary.RandomIntegerInRange` 0 1) (`KismetMathLibrary.RandomIntegerInRange` 2 (`local.LastDoorIndex`)) (`local.bDontUseBraces`)))
  (set `local.RandomDoorSpot` (`KismetMathLibrary.RandomIntegerInRange` 1 (`KismetMathLibrary.SelectInt` (- (`self.LengthOfHouse`) 2) (- (`self.WidthOfHouse`) 2) (or (`|EnumEquality` _houseside "NewEnumerator0") (`|EnumEquality` _houseside "NewEnumerator1")))))
  (bind _structout (setmembers `/Game/Environment/KitBash/Blueprints/STR_MeshWithTransform` :`StructRef` (`|GetArrayItem` (select `/Game/Environment/KitBash/Blueprints/ENUM_HouseSides` (`local.HouseSide`) :`NewEnumerator0` _bottomfloorsides_northwall_3 :`NewEnumerator1` _bottomfloorsides_southwall_3 :`NewEnumerator2` _bottomfloorsides_eastwall_3 :`NewEnumerator3` _bottomfloorsides_westwall_3) (`local.RandomDoorSpot`)) :`Mesh` (`|GetArrayItem` (`self.BottomFloorOptions`) (`local.RandomDoorStyle`))))
  (bind _returnvalue_4 (`AddComponent|NODE_AddStaticMeshComponent-23` :`RelativeTransform` (`.Transform_5_564390C0422EC8ED3F1AFF98228B10FB` (break `/Game/Environment/KitBash/Blueprints/STR_MeshWithTransform` _structout))))
  (`StaticMeshComponent.SetStaticMesh` _returnvalue_4 (break `/Game/Environment/KitBash/Blueprints/STR_MeshWithTransform` _structout))
  (if (`local.bUseDoorCover`)
    (bind _returnvalue_5 (`AddComponent|NODE_AddStaticMeshComponent-21` :`RelativeTransform` (`.Transform_5_564390C0422EC8ED3F1AFF98228B10FB` (break `/Game/Environment/KitBash/Blueprints/STR_MeshWithTransform` _structout))))
    (bind _output_get_3 (set `local.DoorStaticMesh` (`|GetArrayItem` (`self.AboveDoorOptions`) (`KismetMathLibrary.RandomIntegerInRange` 0 1))))
    (`StaticMeshComponent.SetStaticMesh` _returnvalue_5 _output_get_3)
    (`SceneComponent.K2_SetRelativeRotation` _returnvalue_5 (`KismetMathLibrary.MakeRotator` 0.0 0.0 (`KismetMathLibrary.Conv_IntToDouble` (select `/Game/Environment/KitBash/Blueprints/ENUM_HouseSides` (`local.HouseSide`) :`NewEnumerator2` 90 :`NewEnumerator3` 90))) false false)
    (`SceneComponent.SetRelativeScale3D` _returnvalue_5 (`KismetMathLibrary.MakeVector` 1.0 (`KismetMathLibrary.Conv_IntToDouble` (select `/Game/Environment/KitBash/Blueprints/ENUM_HouseSides` (`local.HouseSide`) :`NewEnumerator0` 1 :`NewEnumerator1` -1 :`NewEnumerator2` -1 :`NewEnumerator3` 1)) 1.0))
    (setmembers `/Game/Environment/KitBash/Blueprints/STR_MeshWithTransform` :`StructRef` (select `/Game/Environment/KitBash/Blueprints/ENUM_HouseSides` (`local.HouseSide`) :`NewEnumerator0` _bottomfloordoorcovers_northwall_2 :`NewEnumerator1` _bottomfloordoorcovers_southwall_2 :`NewEnumerator2` _bottomfloordoorcovers_eastwall_2 :`NewEnumerator3` _bottomfloordoorcovers_westwall_2) :`Mesh` (`local.DoorStaticMesh`) :`Transform` (`SceneComponent.GetRelativeTransform` _returnvalue_5))
    (else
      (setmembers `/Game/Environment/KitBash/Blueprints/STR_MeshWithTransform` :`StructRef` (select `/Game/Environment/KitBash/Blueprints/ENUM_HouseSides` (`local.HouseSide`) :`NewEnumerator0` _bottomfloordoorcovers_northwall :`NewEnumerator1` _bottomfloordoorcovers_southwall :`NewEnumerator2` _bottomfloordoorcovers_eastwall :`NewEnumerator3` _bottomfloordoorcovers_westwall) :`Mesh` null :`Transform` "0.000000,0.000000,0.000000|0.000000,0.000000,-0.000000|1.000000,1.000000,1.000000"))))

(fn `CreateUpperLevels`
  (params (HouseSide :type "/Game/Environment/KitBash/Blueprints/ENUM_HouseSides Enum" :default "NewEnumerator0"))
  (locals (bDontUseBraces :type Boolean) (bUseOffset :type Boolean) (NumTilesToMake :type Integer) (Index :type Integer) (RelativeTransform :type "Transform Structure"))
  (bind _numtilestomake (`local.NumTilesToMake`))
  (bind (_bottomfloorsides_northwall _bottomfloorsides_southwall _bottomfloorsides_eastwall _bottomfloorsides_westwall) (break `/Game/Environment/KitBash/Blueprints/STR_SideArrays` (`self.BottomFloorSides`)))
  (bind (_bottomfloorsides_northwall_2 _bottomfloorsides_southwall_2 _bottomfloorsides_eastwall_2 _bottomfloorsides_westwall_2) (break `/Game/Environment/KitBash/Blueprints/STR_SideArrays` (`self.BottomFloorSides`)))
  (bind _returnvalue (- (`self.LengthOfHouse`) 1))
  (bind _returnvalue_2 (- (`self.WidthOfHouse`) 1))
  (bind _output_mesh (break `/Game/Environment/KitBash/Blueprints/STR_MeshWithTransform` (`|GetArrayItem` (select `/Game/Environment/KitBash/Blueprints/ENUM_HouseSides` (`local.HouseSide`) :`NewEnumerator0` _bottomfloorsides_northwall_2 :`NewEnumerator1` _bottomfloorsides_southwall_2 :`NewEnumerator2` _bottomfloorsides_eastwall_2 :`NewEnumerator3` _bottomfloorsides_westwall_2) (`local.Index`))))
  ;[0 1 0] Set all of the random variables for side variations
  (set `local.bDontUseBraces` (`KismetMathLibrary.RandomBool`))
  (bind _output_get (set `local.bUseOffset` (`KismetMathLibrary.RandomBoolWithWeight` 0.333)))
  (`self.AddCornerPost` (`local.HouseSide`))
  (`KismetArrayLibrary.Array_Set` (`self.BottomFloorSideIsOffset`) (select `/Game/Environment/KitBash/Blueprints/ENUM_HouseSides` (`local.HouseSide`) :`NewEnumerator1` 1 :`NewEnumerator2` 2 :`NewEnumerator3` 3) _output_get)
  ;[0 1 0] Set the number of tiles to make based on the cardinal direction and the corresponding length or width
  (switch `/Game/Environment/KitBash/Blueprints/ENUM_HouseSides` (`local.HouseSide`)
    (:`NewEnumerator0`
      (set `local.NumTilesToMake` _returnvalue))
    (:`NewEnumerator1`
      (set `local.NumTilesToMake` _returnvalue))
    (:`NewEnumerator2`
      (set `local.NumTilesToMake` _returnvalue_2))
    (:`NewEnumerator3`
      (set `local.NumTilesToMake` _returnvalue_2)))
  (for _index (range (+ _numtilestomake 1))
    (set `local.Index` _index)
    (bind _transform (`self.SetTransformFromHouseSide` (`local.HouseSide`) (`local.Index`) (`local.bUseOffset`) _numtilestomake))
    (bind _output_get_2 (set `local.RelativeTransform` _transform))
    (bind _returnvalue_3 (`AddComponent|NODE_AddStaticMeshComponent-25` :`RelativeTransform` _output_get_2))
    (`|ExecutionSequence`
      (:`then_0`
        ;[0 1 0] Add the random tile to the correct BottomFloorSides array
        (`KismetArrayLibrary.Array_Add` (select `/Game/Environment/KitBash/Blueprints/ENUM_HouseSides` (`local.HouseSide`) :`NewEnumerator0` _bottomfloorsides_northwall :`NewEnumerator1` _bottomfloorsides_southwall :`NewEnumerator2` _bottomfloorsides_eastwall :`NewEnumerator3` _bottomfloorsides_westwall) (make `/Game/Environment/KitBash/Blueprints/STR_MeshWithTransform` (`|GetArrayItem` (`self.BottomFloorOptions`) (`KismetMathLibrary.SelectInt` 4 5 (`local.bDontUseBraces`))) (`local.RelativeTransform`))))
      (:`then_1`
        ;[0 1 0] Set the static mesh just added to the StaticMeshComponent array to the one added to the BottomFloorSides array
        (`StaticMeshComponent.SetStaticMesh` _returnvalue_3 _output_mesh)))))

(fn `GetMeshHeight`
  (params (Mesh :type "StaticMesh Object Reference"))
  (returns (Height :type "Float (double-precision)"))
  (bind _returnvalue (`StaticMesh.GetBoundingBox` Mesh))
  (return (- (.z (`.Max` (break `Box` _returnvalue))) (.z (break `Box` _returnvalue)))))

(fn `GetMeshLength`
  (params (Mesh :type "StaticMesh Object Reference"))
  (returns (Length :type "Float (double-precision)"))
  (bind _returnvalue (`StaticMesh.GetBoundingBox` Mesh))
  (return (- (.x (`.Max` (break `Box` _returnvalue))) (.x (break `Box` _returnvalue)))))

(fn `ResetVariables`
  (set `self.BottomFloorSides` (struct))
  (set `self.CurrentFloor` 1))

(fn `SetTransformFromHouseSide`
  (params (HouseSide :type "/Game/Environment/KitBash/Blueprints/ENUM_HouseSides Enum" :default "NewEnumerator0") (CurrentIndex :type Integer) (bUseOffset :type Boolean) (TilesToMake :type Integer))
  (returns (Transform :type "Transform Structure"))
  (locals (RelativeTransform :type "Transform Structure") (Index :type Integer) (OffsetAmount :type Integer :default 0))
  (set `local.Index` CurrentIndex)
  (set `local.OffsetAmount` (`KismetMathLibrary.SelectInt` 100 0 (and (not (or (< (`local.Index`) 1) (>= (`local.Index`) (`local.TilesToMake`)))) (`local.bUseOffset`))))
  (switch `/Game/Environment/KitBash/Blueprints/ENUM_HouseSides` HouseSide
    (:`NewEnumerator0`
      (set `local.RelativeTransform` (`KismetMathLibrary.MakeTransform` (`KismetMathLibrary.MakeVector` (`KismetMathLibrary.Conv_IntToDouble` (* (`local.Index`) (`self.LengthOfOneTile`))) (`KismetMathLibrary.Conv_IntToDouble` (+ (* (`self.WidthOfHouse`) (`self.LengthOfOneTile`)) (`local.OffsetAmount`))) (`KismetMathLibrary.Conv_IntToDouble` (* (`self.HeightOfOneTile`) (- (`self.CurrentFloor`) 1)))))))
    (:`NewEnumerator1`
      (set `local.RelativeTransform` (`KismetMathLibrary.MakeTransform` (`KismetMathLibrary.MakeVector` (`KismetMathLibrary.Conv_IntToDouble` (* (`local.Index`) (`self.LengthOfOneTile`))) (`KismetMathLibrary.Conv_IntToDouble` (* (`local.OffsetAmount`) -1)) (`KismetMathLibrary.Conv_IntToDouble` (* (`self.HeightOfOneTile`) (- (`self.CurrentFloor`) 1)))))))
    (:`NewEnumerator2`
      (set `local.RelativeTransform` (`KismetMathLibrary.MakeTransform` (`KismetMathLibrary.MakeVector` (`KismetMathLibrary.Conv_IntToDouble` (+ (* (`self.LengthOfHouse`) (`self.LengthOfOneTile`)) (`local.OffsetAmount`))) (`KismetMathLibrary.Conv_IntToDouble` (* (`local.Index`) (`self.LengthOfOneTile`))) (`KismetMathLibrary.Conv_IntToDouble` (* (`self.HeightOfOneTile`) (- (`self.CurrentFloor`) 1)))) (`KismetMathLibrary.MakeRotator` 0.0 0.0 90.0))))
    (:`NewEnumerator3`
      (set `local.RelativeTransform` (`KismetMathLibrary.MakeTransform` (`KismetMathLibrary.MakeVector` (`KismetMathLibrary.Conv_IntToDouble` (* (`local.OffsetAmount`) -1)) (`KismetMathLibrary.Conv_IntToDouble` (* (`local.Index`) (`self.LengthOfOneTile`))) (`KismetMathLibrary.Conv_IntToDouble` (* (`self.HeightOfOneTile`) (- (`self.CurrentFloor`) 1)))) (`KismetMathLibrary.MakeRotator` 0.0 0.0 90.0)))))
  (return (`local.RelativeTransform`)))

(fn `UploadBottomFloorSide`
  (params (HouseSides :type "/Game/Environment/KitBash/Blueprints/ENUM_HouseSides Enum" :default "NewEnumerator0"))
  (bind (_bottomfloorsides_northwall _bottomfloorsides_southwall _bottomfloorsides_eastwall _bottomfloorsides_westwall) (break `/Game/Environment/KitBash/Blueprints/STR_SideArrays` (`self.BottomFloorSides`)))
  (bind (_bottomfloordoorcovers_northwall _bottomfloordoorcovers_southwall _bottomfloordoorcovers_eastwall _bottomfloordoorcovers_westwall) (break `/Game/Environment/KitBash/Blueprints/STR_SideTile` (`self.BottomFloorDoorCovers`)))
  (bind (_returnvalue_mesh _returnvalue_transform) (break `/Game/Environment/KitBash/Blueprints/STR_MeshWithTransform` (select `/Game/Environment/KitBash/Blueprints/ENUM_HouseSides` (`local.HouseSides`) :`NewEnumerator0` _bottomfloordoorcovers_northwall :`NewEnumerator1` _bottomfloordoorcovers_southwall :`NewEnumerator2` _bottomfloordoorcovers_eastwall :`NewEnumerator3` _bottomfloordoorcovers_westwall)))
  (for _array_element (select `/Game/Environment/KitBash/Blueprints/ENUM_HouseSides` (`local.HouseSides`) :`NewEnumerator0` _bottomfloorsides_northwall :`NewEnumerator1` _bottomfloorsides_southwall :`NewEnumerator2` _bottomfloorsides_eastwall :`NewEnumerator3` _bottomfloorsides_westwall)
    (bind _returnvalue (`AddComponent|NODE_AddStaticMeshComponent-17` :`RelativeTransform` (`.Transform_5_564390C0422EC8ED3F1AFF98228B10FB` (break `/Game/Environment/KitBash/Blueprints/STR_MeshWithTransform` _array_element))))
    (`StaticMeshComponent.SetStaticMesh` _returnvalue (break `/Game/Environment/KitBash/Blueprints/STR_MeshWithTransform` _array_element))
    (`self.AddCornerPost` (`local.HouseSides`)))
  (`|ExecutionSequence`
    (:`then_0`
      (bind _returnvalue_2 (`AddComponent|NODE_AddStaticMeshComponent-24` :`RelativeTransform` _returnvalue_transform))
      (`StaticMeshComponent.SetStaticMesh` _returnvalue_2 _returnvalue_mesh))
    (:`then_1`
      (if (`|GetArrayItem` (`self.BottomFloorSideIsOffset`) (select `/Game/Environment/KitBash/Blueprints/ENUM_HouseSides` (`local.HouseSides`) :`NewEnumerator1` 1 :`NewEnumerator2` 2 :`NewEnumerator3` 3))
        (`self.AddOffsetMeshes` (`local.HouseSides`))))))

(fn `UserConstructionScript`
  (bind _output (`|GetArrayItem` (`self.BottomFloorOptions`)))
  (set `self.LengthOfOneTile` (`KismetMathLibrary.FTrunc` (`self.GetMeshLength` _output)))
  (set `self.HeightOfOneTile` (`KismetMathLibrary.FTrunc` (`self.GetMeshHeight` _output)))
  (if (`self.bStopLogic`)
    (for _array_element (`self.HouseSideOptions`)
      (`self.UploadBottomFloorSide` _array_element))
    (else
      (`|ExecutionSequence`
        (:`then_0`
          (`self.ResetVariables`))
        (:`then_1`
          (for _array_element_2 (`self.HouseSideOptions`)
            (`self.CreateBottomFloorSide` _array_element_2)
            (`self.AddOffsetMeshes` _array_element_2)
            (for _ (range (`self.HeightOfHouse`))
              _)))))))